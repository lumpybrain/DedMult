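; Planet command component that shows a stand-in ship above its owner while a build-ship command is registered.
; On registration outside turn processing, it resets a fade timer, enables tick and spawns an unattached fake ship at a Z offset, avoiding scale issues, with the owner's team.
; Unregistering that command type disables tick and destroys the fake ship.
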(event EventBeginPlay
  (Components|Tick|SetComponentTickEnabled false)
  (EventDispatchers|BindEventtoOnCommandRegistered (EventDispatchers|CreateEvent :!event InitializeBuild))
  (EventDispatchers|BindEventtoOnCommandUnregistered (EventDispatchers|CreateEvent :!event CommandUnregistered)))

(fn InitializeBuild
  (params (NewCommand :type DM%20Command%20Object%20Reference))
  (bind _returnvalue (Components|GetOwner))
  (bind _returnvalue_2 (Transformation|GetActorLocation _returnvalue))
  (Utilities|Casting|CastToDMCommand_BuildShip NewCommand
    (:then
      (bind _asdmgame_state (Utilities|Casting|CastToDMGameState (Game|GetGameState))
        (:then
          (bind _returnvalue_3 (Class|DMGameState|IsProcessingATurn _asdmgame_state))
          (if (not _returnvalue_3)
            (Variables|ActiveBuildVis|SetFadeTimer 0.0)
            (Components|Tick|SetComponentTickEnabled true)
            ;[0.15 0.15 0.15 0.5] Note: We're not attaching so we don't worry about scale
            (bind _returnvalue_4 (Game|SpawnActorfromClass (Variables|BuildVisualizationCustomization|GetFakeShipClass) (Math|Transform|MakeTransform (Math|Vector|MakeVector (.x _returnvalue_2) (.y _returnvalue_2) (+ (.z _returnvalue_2) (Variables|/Script/MultStrat.CommandsDataAsset|GetShipSpawnZOffset (Variables|/Script/MultStrat.DMGameState|GetCommandsData _asdmgame_state)))) (Transformation|GetActorRotation _returnvalue) "1.000000,1.000000,1.000000") "Undefined" "MultiplyWithRoot" 0 0))
            (bind _output_get (Variables|ActiveBuildVis|SetActiveFade _returnvalue_4))
            (Class|DMTeamComponent|SetTeam (Variables|/Script/MultStrat.DMBaseGalaxyObject|GetTeamComponent _output_get) (Class|DMTeamComponent|GetTeam (Actor|GetComponentbyClass (Components|GetOwner) "/Script/MultStrat.DMTeamComponent")))))
        (:CastFailed
          (Class|DMLogsBlueprintLibrary|PrintLogCommandsError (Utilities|String|Append (Utilities|GetDisplayName (Components|GetOwner)) " unable to get game state in Planet Commands Component InitializeBuild"))
          (return))))
    (:CastFailed
      (return))))

(fn CommandUnregistered
  (params (OldCommand :type DM%20Command%20Object%20Reference))
  (bind _activefade (Variables|ActiveBuildVis|GetActiveFade))
  (Utilities|Casting|CastToDMCommand_BuildShip OldCommand
    (:then
      (Components|Tick|SetComponentTickEnabled false)
      (Utilities|IsValid _activefade
        (:Is%20Valid
          (Actor|DestroyActor _activefade))))
    (:CastFailed
      (return))))