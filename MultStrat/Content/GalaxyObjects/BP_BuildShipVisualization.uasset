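; BP_BuildShipVisualization is a galaxy object that, going by its name, visualizes a ship under construction with a pulsing translucent look.
; Its construction script sets MI_BuildingShip as the material class, then runs the parent construction script.
; Each tick accumulates a fade timer and drives the dynamic material's Opacity through a cosine wave, oscillating between the minimum and maximum transparency at the configured fade speed.
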(event EventTick
  (params (DeltaSeconds :type Float%20%28single-precision%29))
  (bind _output_get (Variables|Default|SetFadeTimer (+ DeltaSeconds (Variables|Default|GetFadeTimer))))
  (Rendering|Material|SetScalarParameterValue (Variables|Default|GetDynamicMaterial) "Opacity" (+ (Variables|Default|GetMinTransparancy) (* (- (Variables|Default|GetMaxTransparancy) (Variables|Default|GetMinTransparancy)) (+ (* (Math|Trig|Cos(Radians) (* _output_get (Variables|Default|GetFadeSpeed))) -1.0 0.5) 0.5))) :!class /Script/Engine.MaterialInstanceDynamic))

(fn ConstructionScript
  (Variables|Default|SetMaterialClass "/Game/Art/Materials/MI_BuildingShip.MI_BuildingShip")
  (|CallParentFunction))