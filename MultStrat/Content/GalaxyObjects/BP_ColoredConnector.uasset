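; BP_ColoredConnector is a galaxy-object actor that draws a pulsing, team-colored link from the starting node's ship to an ending node.
; InitializeSplineMesh rotates the whole actor along the link so X suits M_Pulsing's math, then counter-rotates both endpoints to place the spline mesh.
; It applies a dynamic MI_Pulsing instance, setting opacity and the color DMGameState returns for that ship's team.
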(event EventBeginPlay)

(event Collision|EventActorBeginOverlap
  (params (OtherActor :type Actor%20Object%20Reference)))

(event EventTick
  (params (DeltaSeconds :type Float%20%28single-precision%29)))

(fn ConstructionScript)

(fn InitializeSplineMesh
  (params (StartingNode :type DM%20Galaxy%20Node%20Object%20Reference) (EndingNode :type DM%20Galaxy%20Node%20Object%20Reference))
  (bind _returnvalue (Transformation|GetActorLocation EndingNode))
  (bind _returnvalue_2 (Class|DMGalaxyNode|GetShip StartingNode))
  (bind _splinemeshcomponent (Variables|Default|GetSplineMeshComponent))
  (bind _returnvalue_3 (Transformation|GetActorLocation _returnvalue_2))
  (bind _returnvalue_4 (- _returnvalue _returnvalue_3))
  (bind _returnvalue_5 (Math|Vector|Normalize _returnvalue_4))
  (bind _returnvalue_6 (Math|Conversions|ToQuaternion(Rotator) _returnvalue_5))
  (bind _returnvalue_7 (Class|KismetMathLibrary|QuatRotator _returnvalue_6))
  (bind _returnvalue_8 (Class|KismetMathLibrary|NegateRotator _returnvalue_7))
  ;[0.15 0.15 0.15 0.5] Make our spline, but make the whole actor rotate so that the X value is valid during M_Pulsing's math
  (Transformation|SetActorRotation _returnvalue_7)
  (SplineMesh|SetStartandEnd _splinemeshcomponent (Math|Vector|RotateVector _returnvalue_3 _returnvalue_8) "1.000000,0.000000,0.000000" (Math|Vector|RotateVector _returnvalue _returnvalue_8) "1.000000,0.000000,0.000000" true :!class /Script/Engine.SplineMeshComponent)
  (SplineMesh|SetForwardAxis _splinemeshcomponent "Z" true)
  ;[0.15 0.15 0.15 0.5] Set up the material
  (bind _returnvalue_9 (Rendering|Material|CreateDynamicMaterialInstance "/Game/Art/Materials/MI_Pulsing.MI_Pulsing" "None" "None" :!class /Script/Engine.KismetMaterialLibrary))
  (Rendering|Material|SetMaterial (Variables|Default|GetSplineMeshComponent) 0 _returnvalue_9)
  (bind _asdmgame_state (Utilities|Casting|CastToDMGameState (Game|GetGameState)))
  (bind _output (Class|DMGameState|GetColorforTeam _asdmgame_state (Class|DMTeamComponent|GetTeam (Variables|/Script/MultStrat.DMBaseGalaxyObject|GetTeamComponent _returnvalue_2))))
  (Rendering|Material|SetVectorParameterValue _returnvalue_9 "Color" (Math|Conversions|ToLinearColor(Color) _output) :!class /Script/Engine.MaterialInstanceDynamic)
  (Rendering|Material|SetScalarParameterValue _returnvalue_9 "Opacity" (Variables|Default|GetOpacityForSpline) :!class /Script/Engine.MaterialInstanceDynamic))