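; BP_DMPlanet is a galaxy planet whose color shows the player team that controls it.
; The construction script creates a dynamic instance of MI_ControlledPlanet on its static mesh.
; BeginPlay binds to the TeamComponent's team-change event and applies the initial color if the team is valid.
; Both paths set the material's Color parameter from the DMGameState team color, and a team change logs an error if the game state is unavailable.
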(event Custom|Team%20Changed
  (params (ChangedActor :type Actor%20Object%20Reference) (NewTeam :type EDMPlayerTeam%20Enum :default "Invalid"))
  (bind _asdmgame_state (Utilities|Casting|CastToDMGameState (Game|GetGameState))
    (:then
      (bind _output (Class|DMGameState|GetColorforTeam _asdmgame_state NewTeam))
      ;[0.15 0.15 0.15 0.5] Note: Set Linear Color in vector parameter (0->1.0 values), FColor for debug print (0->255 values)
      (Rendering|Material|SetVectorParameterValue (Variables|Default|GetDynamicMaterial) "Color" (Math|Conversions|ToLinearColor(Color) _output) :!class /Script/Engine.MaterialInstanceDynamic))
    (:CastFailed
      (Class|DMLogsBlueprintLibrary|PrintLogTeamsError (Utilities|String|Append (Utilities|GetDisplayName self) " tried to set its color in team changed event, but couldn't get its game state")))))

(event EventBeginPlay
  (bind _teamcomponent (Variables|Default|GetTeamComponent))
  (bind _returnvalue (Class|DMTeamComponent|GetTeam _teamcomponent))
  (EventDispatchers|AssignOnActiveTeamChanged (Variables|Default|GetTeamComponent) (delegate Custom|Team%20Changed))
  (if (Utilities|Enum|NotEqual(Enum) _returnvalue (Utilities|Enum|LiteralenumEDMPlayerTeam "Invalid"))
    (bind _asdmgame_state (Utilities|Casting|CastToDMGameState (Game|GetGameState)))
    (bind _output (Class|DMGameState|GetColorforTeam _asdmgame_state _returnvalue))
    (Rendering|Material|SetVectorParameterValue (Variables|Default|GetDynamicMaterial) "Color" (Math|Conversions|ToLinearColor(Color) _output) :!class /Script/Engine.MaterialInstanceDynamic)))

(fn ConstructionScript
  (bind _returnvalue (Rendering|Material|CreateDynamicMaterialInstance "/Game/Art/Materials/MI_ControlledPlanet.MI_ControlledPlanet" "None" "None" :!class /Script/Engine.KismetMaterialLibrary))
  (bind _output_get (Variables|Default|SetDynamicMaterial _returnvalue))
  (Rendering|Material|SetMaterial (Variables|Default|GetStaticMeshComponent) 0 _output_get))