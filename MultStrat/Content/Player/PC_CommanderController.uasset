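; Player controller for the commander pawn, handling planar movement, orbit camera and click selection.
; Holding right mouse hides the cursor and orbits the pawn around its view point, using a distance to the game plane computed at BeginPlay.
; On release, Tick decays the rotation as inertia, with separate friction while moving to limit motion sickness.
; Left-click traces under the cursor to show or clear galaxy node HUD UI and notify clicked spheres.
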(event Custom|ClickedOnSphere
  (params (ClickSphere :type Clicked%20Sphere%20Object%20Reference))
  (Default|Clickedon ClickSphere self))

(event EventBeginPlay
  (Variables|Default|SetMousePosition (/ (Viewport|GetViewportSize) "(X=2.000000,Y=2.000000)"))
  (CallFunction|ShowMouseCursor)
  (bind _asbp_commander_character (Utilities|Casting|CastToBP_CommanderCharacter (Pawn|GetControlledPawn)))
  (Variables|Default|SetPlayerPawn _asbp_commander_character)
  (Input|AddMappingContext (PlayerController|LocalPlayerSubsystems|GetEnhancedInputLocalPlayerSubsystem) "/Game/Player/Input/IMC_Commander.IMC_Commander" 0 "(bIgnoreAllPressedKeysUntilRelease=True,bForceImmediately=False,bNotifyUserSettings=False)")
  (CallFunction|CalculatePlaneIntersectionDistance))

(event EventTick
  (params (DeltaSeconds :type Float%20%28single-precision%29))
  (if (Utilities|Operators|NotEqual(!=) :A (Variables|CameraSlide|GetCurrentRotationRate) :ErrorTolerance 0.0)
    (if (< (Variables|CameraSlide|GetMinCamMoveSquared) (Math|Vector|VectorLengthSquared (Variables|CameraSlide|GetCurrentRotationRate)))
      ;[0.15 0.15 0.15 0.5] If we're moving, reduce rotation at an increased rate to avoid motion sickness
      (if (> (Math|Vector|VectorLengthSquared (Variables|/Script/Engine.MovementComponent|GetVelocity (Variables|/Script/Engine.Character|GetCharacterMovement (Variables|Default|GetPlayerPawn)))) 0.0)
        (Variables|CameraSlide|SetCurrentRotationRate (* (Variables|CameraSlide|GetCurrentRotationRate) (Variables|CameraSlide|GetMovingRotationFriction)))
        (else
          (Variables|CameraSlide|SetCurrentRotationRate (* (Variables|CameraSlide|GetCurrentRotationRate) (Variables|CameraSlide|GetRotationFriction)))))
      (if (not (Variables|Default|GetRMBHeld))
        (CallFunction|RotateCharacterAroundPlane (.y (Variables|CameraSlide|GetCurrentRotationRate)) (.z (Variables|CameraSlide|GetCurrentRotationRate))))
      (else
        (Variables|CameraSlide|SetCurrentRotationRate (Math|Vector|VectorZero))))))

(event Input|EnhancedActionEvents|EnhancedInputActionIA_Forward
  (params (ActionValue :type Float%20%28double-precision%29) (ElapsedSeconds :type Float%20%28double-precision%29) (TriggeredSeconds :type Float%20%28double-precision%29) (InputAction :type Input%20Action%20Object%20Reference :default "/Game/Player/Input/IA_Forward.IA_Forward"))
  ;[0.15 0.15 0.15 0.5] IA_Forward: Forward and Back on 2D Plane
  (Pawn|Input|AddMovementInput (Variables|Default|GetPlayerPawn) (Class|KismetMathLibrary|VectorNormal2D (Transformation|GetActorForwardVector (Variables|Default|GetPlayerPawn)) 0.0001) ActionValue false))

(event Input|EnhancedActionEvents|EnhancedInputActionIA_Right
  (params (ActionValue :type Float%20%28double-precision%29) (ElapsedSeconds :type Float%20%28double-precision%29) (TriggeredSeconds :type Float%20%28double-precision%29) (InputAction :type Input%20Action%20Object%20Reference :default "/Game/Player/Input/IA_Right.IA_Right"))
  ;[0.15 0.15 0.15 0.5] IA_Right: Right and Left on 2d Plane
  (Pawn|Input|AddMovementInput (Variables|Default|GetPlayerPawn) (Class|KismetMathLibrary|VectorNormal2D (Transformation|GetActorRightVector (Variables|Default|GetPlayerPawn)) 0.0001) ActionValue false))

(event Input|EnhancedActionEvents|EnhancedInputActionIA_EnableRotation
  (params (ActionValue :type Float%20%28double-precision%29) (ElapsedSeconds :type Float%20%28double-precision%29) (TriggeredSeconds :type Float%20%28double-precision%29) (InputAction :type Input%20Action%20Object%20Reference :default "/Game/Player/Input/IA_EnableRotation.IA_EnableRotation"))
  ;[0.15 0.15 0.15 0.5] Right Click to enable camera rotation
  (:Started
    (Variables|Default|SetRMBHeld true)
    (CallFunction|HideMouseCursor))
  (:Canceled
    (Variables|Default|SetRMBHeld false :!label _label)
    (CallFunction|ShowMouseCursor))
  (:Completed
    (goto _label)))

(event Input|EnhancedActionEvents|EnhancedInputActionIA_MouseMovement
  (params (ActionValue :type Vector%202D%20Structure) (ElapsedSeconds :type Float%20%28double-precision%29) (TriggeredSeconds :type Float%20%28double-precision%29) (InputAction :type Input%20Action%20Object%20Reference :default "/Game/Player/Input/IA_MouseMovement.IA_MouseMovement"))
  ;[0.15 0.15 0.15 0.5] If there's mouse movement AND Enable rotation is enabled, rotate around the controller's default plane Z
  (if (Variables|Default|GetRMBHeld)
    (bind _output_get (Variables|CameraSlide|SetCurrentRotationRate (Math|Vector|MakeVector 0.0 (* (Variables|Default|GetPitch%20Rate) (.y ActionValue)) (* (.x ActionValue) (Variables|Default|GetYawRate)))))
    (CallFunction|RotateCharacterAroundPlane (.y _output_get) (.z _output_get))))

(event Input|EnhancedActionEvents|EnhancedInputActionIA_LeftMouseClick
  (params (ActionValue :type Boolean) (ElapsedSeconds :type Float%20%28double-precision%29) (TriggeredSeconds :type Float%20%28double-precision%29) (InputAction :type Input%20Action%20Object%20Reference :default "/Game/Player/Input/IA_LeftMouseClick.IA_LeftMouseClick"))
  (bind _hitresult (Game|Player|GetHitResultUnderCursorbyChannel "TraceTypeQuery1" true))
  ;[0.15 0.15 0.15 0.5] On Left Click
  (:Started
    (Utilities|FlowControl|Sequence
      (:then_0
        (bind _asbp_commander_hud (Utilities|Casting|CastToBP_CommanderHud (HUD|GetHUD)))
        (bind _asdmgalaxy_node (Utilities|Casting|CastToDMGalaxyNode (.hitactor _hitresult))
          (:then
            (Default|SpawnNodeUI _asbp_commander_hud _asdmgalaxy_node))
          (:CastFailed
            (Default|ClearNodeUI _asbp_commander_hud))))
      (:then_1
        ;;[0.15 0.15 0.15 0.5] Clean up later: Check if we clicked a sphere (TODO: Make a clicked interface!)
        (bind _asclicked_sphere (Utilities|Casting|CastToClickedSphere (.hitactor _hitresult)))
        (CallFunction|ClickedonSphere _asclicked_sphere)))))

(fn ConstructionScript)

(fn ShowMouseCursor
  (bind _mouseposition (Variables|Default|GetMousePosition))
  (Variables|Default|SetbShowMouseCursor true)
  (Input|SetInputModeGameandUI self 0 "LockOnCapture" true false)
  (Class|PlayerController|SetMouseLocation (Math|Float|Truncate (.x _mouseposition)) (Math|Float|Truncate (.y _mouseposition))))

(fn HideMouseCursor
  (bind (_locationx _locationy) (Game|Player|GetMousePosition))
  (Variables|Default|SetbShowMouseCursor false)
  (Input|SetInputModeGameOnly self false)
  (Variables|Default|SetMousePosition (Math|Vector2D|MakeVector2D _locationx _locationy)))

(fn RotateCharacterAroundPlane
  (params (PitchMovement :type Float%20%28double-precision%29) (YawMovement :type Float%20%28double-precision%29))
  (bind _playerpawn (Variables|Default|GetPlayerPawn))
  (bind _playerpawn_2 (Variables|Default|GetPlayerPawn))
  (bind _playerpawn_3 (Variables|Default|GetPlayerPawn))
  (bind _returnvalue (Transformation|GetActorRotation _playerpawn))
  (bind _camera (Variables|/Game/Player/BP_CommanderCharacter.BP_CommanderCharacter_C|GetCamera _playerpawn_2))
  (bind _returnvalue_2 (Transformation|GetWorldRotation _camera))
  (bind _output_get (LocalVariables|SetActorLocation (Transformation|GetActorLocation (Variables|Default|GetPlayerPawn))))
  (bind _output_get_2 (LocalVariables|SetCameraFacing (Math|Vector|GetForwardVector (Variables|/Game/Player/BP_CommanderCharacter.BP_CommanderCharacter_C|GetCamera (Variables|Default|GetPlayerPawn)))))
  (LocalVariables|SetIntersectionPoint (+ _output_get (* _output_get_2 (Variables|Default|GetDistanceFromIntersection))))
  ;[0.15 0.15 0.15 0.5] Rotate the Actor
  (Transformation|SetActorRotation _playerpawn (Math|Rotator|MakeRotator (.roll _returnvalue) (+ PitchMovement (.pitch _returnvalue)) (+ YawMovement (.yaw _returnvalue))) true)
  ;[0.15 0.15 0.15 0.5] Set the actors Location
  (Transformation|SetActorLocation _playerpawn_3 (+ (LocalVariables|GetIntersectionPoint) (* (Math|Vector|GetForwardVector (Math|Rotator|MakeRotator (.roll _returnvalue_2) (+ (.pitch _returnvalue_2) 1.8e+02) (.yaw _returnvalue_2))) (Variables|Default|GetDistanceFromIntersection))) false false)
  (Default|SetReplicatedActorLocation _playerpawn_3 (+ (LocalVariables|GetIntersectionPoint) (* (Math|Vector|GetForwardVector (Math|Rotator|MakeRotator (.roll _returnvalue_2) (+ (.pitch _returnvalue_2) 1.8e+02) (.yaw _returnvalue_2))) (Variables|Default|GetDistanceFromIntersection)))))

(fn CalculatePlaneIntersectionDistance
  (LocalVariables|SetActorLocation (Transformation|GetActorLocation (Variables|Default|GetPlayerPawn)))
  (LocalVariables|SetCameraFacing (Math|Vector|GetForwardVector (Variables|/Game/Player/BP_CommanderCharacter.BP_CommanderCharacter_C|GetCamera (Variables|Default|GetPlayerPawn))))
  (Variables|Default|SetDistanceFromIntersection (Math|Vector|Distance(Vector) (Math|Vector|MakeVector (+ (.x (* (LocalVariables|GetCameraFacing) (/ (- (Variables|Default|GetGamePlaneZ) (.z (LocalVariables|GetActorLocation))) (.z (LocalVariables|GetCameraFacing))))) (.x (LocalVariables|GetActorLocation))) (+ (.y (* (LocalVariables|GetCameraFacing) (/ (- (Variables|Default|GetGamePlaneZ) (.z (LocalVariables|GetActorLocation))) (.z (LocalVariables|GetCameraFacing))))) (.y (LocalVariables|GetActorLocation))) (Variables|Default|GetGamePlaneZ)) (Transformation|GetActorLocation (Variables|Default|GetPlayerPawn)))))